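; BP_Cube is an actor Blueprint that acts as a mouse-click debug probe for surface normals.
; It enables input on BeginPlay, and left mouse presses fetch the player controller from the input device.
; A Visibility trace under the cursor supplies the hit normal, whose X, Y and Z components are printed as text.
; A check that the hit actor is the cube itself is unconnected, so printing is not limited to it.
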(event `InputAction|mouseLeft`
  (params (Key :type "Key Structure"))
  (:`Pressed`
    (`KismetSystemLibrary.PrintText` (`KismetTextLibrary.Conv_DoubleToText` (.x (`.Normal` (`GameplayStatics.BreakHitResult` (`PlayerController.GetHitResultUnderCursorByChannel` (stale _returnvalue) "TraceTypeQuery1" false)))) "HalfToEven"))))

(event `InputAction|mouseLeft`
  (params (Key :type "Key Structure"))
  (:`Pressed`
    (`KismetSystemLibrary.PrintText` (`KismetTextLibrary.Conv_DoubleToText` (.z (`.Normal` (`GameplayStatics.BreakHitResult` (`PlayerController.GetHitResultUnderCursorByChannel` (stale _returnvalue) "TraceTypeQuery1" false)))) "HalfToEven"))))

(event `InputAction|mouseLeft`
  (params (Key :type "Key Structure"))
  (:`Pressed`
    (`KismetSystemLibrary.PrintText` (`KismetTextLibrary.Conv_DoubleToText` (.y (`.Normal` (`GameplayStatics.BreakHitResult` (`PlayerController.GetHitResultUnderCursorByChannel` (stale _returnvalue) "TraceTypeQuery1" false)))) "HalfToEven"))))

(event `self.ReceiveBeginPlay`
  (`self.EnableInput` null))

(event `InputAction|mouseLeft`
  (params (Key :type "Key Structure"))
  (:`Pressed`
    (bind _returnvalue (`InputDeviceLibrary.GetPlayerControllerFromInputDevice` (struct)))))

(fn `UserConstructionScript`)
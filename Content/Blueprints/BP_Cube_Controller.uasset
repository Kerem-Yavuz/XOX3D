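; Player controller for a cube-based X/O game that handles mouse rotation, board reset and score printout.
; Left click stores the actor under the cursor, and Tick rotates it by mouse delta while dragging, alongside a Clicked flag for other Blueprints.
; BeginPlay caches Cube_BP and the BP_XOX pawn; R restores six face mesh arrays and clears the pawn's board arrays and points.
; Tab prints scores, and 1 prints array values.
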(event `self.ReceiveTick`
  (params (DeltaSeconds :type "Float (single-precision)"))
  (bind (_deltax _deltay) (`self.GetInputMouseDelta`))
  ;[1 1 1] same with the bottom one but checks validity of left click every tick
  (if (`self.IsDragging`) :!label _label
    (`/Engine/EditorBlueprintResources/StandardMacros.IsValid` (stale `Key|LeftMouseButton` _output_get) :!label _label_2 ; checks for validity of object
      (:`Is Valid`
        (`self.K2_AddActorWorldRotation` (stale `Key|LeftMouseButton` _output_get) (`KismetMathLibrary.MakeRotator` 0.0 (* -3.0 _deltay) (* -3.0 _deltax)) false false)))))

(event `Key|LeftMouseButton`
  (params (Key :type "Key Structure"))
  ;[1 1 1] Diğer BPlerde Kullanıyoruz
  (:`Pressed`
    (set `self.clicked` true))
  (:`Released`
    (set `self.clicked` false)))

(event `Key|LeftMouseButton`
  (params (Key :type "Key Structure"))
  ;[1 1 1] same with the bottom one but checks validity of left click every tick
  (:`Pressed`
    (set `self.IsDragging` true)
    (goto _label))
  (:`Released`
    (set `self.IsDragging` false)
    (goto _label)))

(event `Key|LeftMouseButton`
  (params (Key :type "Key Structure"))
  ;[1 1 1] checks if mouse dragged
  (:`Pressed`
    (set `self.IsDragging` true)
    (if (`self.IsDragging`) :!label _label_3
      ;[1 1 1] gets the target
      (bind _output_get (set `self.CubeReference` (`.HitActor` (`GameplayStatics.BreakHitResult` (`self.GetHitResultUnderCursorByChannel` "TraceTypeQuery1")))))
      (goto _label_2)))
  (:`Released`
    (set `self.IsDragging` false)
    (goto _label_3)))

(event `self.ReceiveBeginPlay`
  (set `self.bShowMouseCursor` true)
  ;[1 1 1] Resets all the cube when R Clicked
  (bind _outactors (`GameplayStatics.GetAllActorsOfClass` "/Game/Blueprints/Cube_BP.Cube_BP_C"))
  (for _array_element _outactors
    (bind _ascube_bp (cast `/Game/Blueprints/Cube_BP` _array_element)))
  (bind _asbp_xox (cast `/Game/Blueprints/BP_XOX` (`self.K2_GetPawn` (`GameplayStatics.GetPlayerController` 0)))))

(event `InputAction|keyboardR`
  (params (Key :type "Key Structure"))
  ;[1 1 1] Resets all the cube when R Clicked
  (:`Pressed`
    (`self.ResetFunction` (`/Game/Blueprints/Cube_BP.dogu_Array` (stale `self.ReceiveBeginPlay` _ascube_bp)) (`/Game/Blueprints/Cube_BP.Batı_Array` (stale `self.ReceiveBeginPlay` _ascube_bp)) (`/Game/Blueprints/Cube_BP.Alt_Array` (stale `self.ReceiveBeginPlay` _ascube_bp)) (`/Game/Blueprints/Cube_BP.Ust_Array` (stale `self.ReceiveBeginPlay` _ascube_bp)) (`/Game/Blueprints/Cube_BP.KuzeyTaraf_Array` (stale `self.ReceiveBeginPlay` _ascube_bp)) (`/Game/Blueprints/Cube_BP.GuneyTaraf_Array` (stale `self.ReceiveBeginPlay` _ascube_bp)) (`/Game/Blueprints/BP_XOX.stopArray` (stale `self.ReceiveBeginPlay` _asbp_xox)) (`/Game/Blueprints/BP_XOX.AltArray` (stale `self.ReceiveBeginPlay` _asbp_xox)) (`/Game/Blueprints/BP_XOX.ÜstArray` (stale `self.ReceiveBeginPlay` _asbp_xox)) (`/Game/Blueprints/BP_XOX.KuzeyArray` (stale `self.ReceiveBeginPlay` _asbp_xox)) (`/Game/Blueprints/BP_XOX.GuneyArray` (stale `self.ReceiveBeginPlay` _asbp_xox)) (`/Game/Blueprints/BP_XOX.DoguArray` (stale `self.ReceiveBeginPlay` _asbp_xox)) (`/Game/Blueprints/BP_XOX.BatıArray` (stale `self.ReceiveBeginPlay` _asbp_xox)))
    (set `/Game/Blueprints/BP_XOX.oPoints` 0 (stale `self.ReceiveBeginPlay` _asbp_xox))
    (set `/Game/Blueprints/BP_XOX.xPoints` 0 (stale `self.ReceiveBeginPlay` _asbp_xox))))

(event `InputAction|keyboardTab`
  (params (Key :type "Key Structure"))
  (:`Pressed`
    (`KismetSystemLibrary.PrintString` "O Points:")
    (`KismetSystemLibrary.PrintString` (`KismetStringLibrary.Conv_IntToString` (`/Game/Blueprints/BP_XOX.oPoints` (stale `self.ReceiveBeginPlay` _asbp_xox))) true true (struct :`R` 0.96 :`A` 1.0))
    (`KismetSystemLibrary.PrintString` "X Points:")
    (`KismetSystemLibrary.PrintString` (`KismetStringLibrary.Conv_IntToString` (`/Game/Blueprints/BP_XOX.xPoints` (stale `self.ReceiveBeginPlay` _asbp_xox))))))

(event `Key|One`
  (params (Key :type "Key Structure"))
  (:`Pressed`
    (for _array_element (`.IntArray_26_C3AD429141D04837589D8DB7D3522A40` (break `/Game/Blueprints/ArrayStruct` (`|GetArrayItem` (`/Game/Blueprints/BP_XOX.ArrayStruct` (stale `self.ReceiveBeginPlay` _asbp_xox)))))
      (`KismetSystemLibrary.PrintText` (`KismetTextLibrary.Conv_IntToText` _array_element)))))

(fn `ResetFunction`
  (params (Dogu :type "Array of PrimitiveComponent Object Reference") (`Batı` :type "Array of PrimitiveComponent Object Reference") (Alt :type "Array of PrimitiveComponent Object Reference") (`Üst` :type "Array of PrimitiveComponent Object Reference") (Kuzey :type "Array of PrimitiveComponent Object Reference") (Guney :type "Array of PrimitiveComponent Object Reference") (StopArray :type "Array of Boolean") (Altnumber :type "Array of Integer") (`ÜstNumber` :type "Array of Integer") (KuzeyNumber :type "Array of Integer") (GuneyNumber :type "Array of Integer") (DoguNumber :type "Array of Integer") (`BatıNumber` :type "Array of Integer"))
  (for _array_element Dogu
    (bind _asstatic_mesh_component (cast `StaticMeshComponent` _array_element))
    (`StaticMeshComponent.SetStaticMesh` _asstatic_mesh_component "/Engine/BasicShapes/Cube.Cube")
    (`PrimitiveComponent.SetMaterial` _asstatic_mesh_component 0 "/Game/Materials/Glass.Glass"))
  (for _array_element_2 `Batı`
    (bind _asstatic_mesh_component_2 (cast `StaticMeshComponent` _array_element_2))
    (`StaticMeshComponent.SetStaticMesh` _asstatic_mesh_component_2 "/Engine/BasicShapes/Cube.Cube")
    (`PrimitiveComponent.SetMaterial` _asstatic_mesh_component_2 0 "/Game/Materials/Glass.Glass"))
  (for _array_element_3 Alt
    (bind _asstatic_mesh_component_3 (cast `StaticMeshComponent` _array_element_3))
    (`StaticMeshComponent.SetStaticMesh` _asstatic_mesh_component_3 "/Engine/BasicShapes/Cube.Cube")
    (`PrimitiveComponent.SetMaterial` _asstatic_mesh_component_3 0 "/Game/Materials/Glass.Glass"))
  (for _array_element_4 `Üst`
    (bind _asstatic_mesh_component_4 (cast `StaticMeshComponent` _array_element_4))
    (`StaticMeshComponent.SetStaticMesh` _asstatic_mesh_component_4 "/Engine/BasicShapes/Cube.Cube")
    (`PrimitiveComponent.SetMaterial` _asstatic_mesh_component_4 0 "/Game/Materials/Glass.Glass"))
  (for _array_element_5 Kuzey
    (bind _asstatic_mesh_component_5 (cast `StaticMeshComponent` _array_element_5))
    (`StaticMeshComponent.SetStaticMesh` _asstatic_mesh_component_5 "/Engine/BasicShapes/Cube.Cube")
    (`PrimitiveComponent.SetMaterial` _asstatic_mesh_component_5 0 "/Game/Materials/Glass.Glass"))
  (for _array_element_6 Guney
    (bind _asstatic_mesh_component_6 (cast `StaticMeshComponent` _array_element_6))
    (`StaticMeshComponent.SetStaticMesh` _asstatic_mesh_component_6 "/Engine/BasicShapes/Cube.Cube")
    (`PrimitiveComponent.SetMaterial` _asstatic_mesh_component_6 0 "/Game/Materials/Glass.Glass"))
  (for (_ _array_index) StopArray
    (`KismetArrayLibrary.Array_Set` StopArray _array_index))
  (for (_ _array_index_2) Altnumber
    (`KismetArrayLibrary.Array_Set` Altnumber _array_index_2))
  (for (_ _array_index_3) `ÜstNumber`
    (`KismetArrayLibrary.Array_Set` `ÜstNumber` _array_index_3))
  (for (_ _array_index_4) KuzeyNumber
    (`KismetArrayLibrary.Array_Set` KuzeyNumber _array_index_4))
  (for (_ _array_index_5) GuneyNumber
    (`KismetArrayLibrary.Array_Set` GuneyNumber _array_index_5))
  (for (_ _array_index_6) DoguNumber
    (`KismetArrayLibrary.Array_Set` DoguNumber _array_index_6))
  (for (_ _array_index_7) `BatıNumber`
    (`KismetArrayLibrary.Array_Set` `BatıNumber` _array_index_7)))

(fn `UserConstructionScript`)
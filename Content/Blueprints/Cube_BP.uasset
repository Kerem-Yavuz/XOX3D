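; Cube Blueprint that organizes 54 pieces into six sides of nine, a layout resembling a Rubik's cube.
; On BeginPlay it enables click events on the first player controller and fills one array per side, using Turkish direction names.
; Each array lists that side's pieces from 9 down to 1.
; No click handling or rotation logic exists yet, and the construction script and macro are empty.
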(event `self.ReceiveBeginPlay`
  (set `PlayerController.bEnableClickEvents` true (`GameplayStatics.GetPlayerController` 0))
  (set `self.GuneyTaraf_Array` (`|MakeArray` (`self.Cube9_ön`) (`self.Cube8_ön`) (`self.Cube7_ön`) (`self.Cube6_ön`) (`self.Cube5_ön`) (`self.Cube4_ön`) (`self.Cube3_ön`) (`self.Cube2_ön`) (`self.Cube1_ön`)))
  (set `self.KuzeyTaraf_Array` (`|MakeArray` (`self.Cube9_arka`) (`self.Cube8_arka`) (`self.Cube7_arka`) (`self.Cube6_arka`) (`self.Cube5_arka`) (`self.Cube4_arka`) (`self.Cube3_arka`) (`self.Cube2_arka`) (`self.Cube1_ arka`)))
  (set `self.dogu_Array` (`|MakeArray` (`self.Cube9_Sag`) (`self.Cube8_Sag`) (`self.Cube7_Sag`) (`self.Cube6_Sag`) (`self.Cube5_Sag`) (`self.Cube4_Sag`) (`self.Cube3_Sag`) (`self.Cube2_Sag`) (`self.Cube1_Sag`)))
  (set `self.Batı_Array` (`|MakeArray` (`self.Cube9_Sol`) (`self.Cube8_Sol`) (`self.Cube7_Sol`) (`self.Cube6_Sol`) (`self.Cube5_Sol`) (`self.Cube4_Sol`) (`self.Cube3_Sol`) (`self.Cube2_Sol`) (`self.Cube1_Sol`)))
  (set `self.Ust_Array` (`|MakeArray` (`self.Cube9_Üst`) (`self.Cube8_Üst`) (`self.Cube7_Üst`) (`self.Cube6_Üst`) (`self.Cube5_Üst`) (`self.Cube4_Üst`) (`self.Cube3_Üst`) (`self.Cube2_Üst`) (`self.Cube1_Üst`)))
  (set `self.Alt_Array` (`|MakeArray` (`self.Cube9_Alt`) (`self.Cube8_Alt`) (`self.Cube7_Alt`) (`self.Cube6_Alt`) (`self.Cube5_Alt`) (`self.Cube4_Alt`) (`self.Cube3_Alt`) (`self.Cube2_Alt`) (`self.Cube1_alt`))))

(fn `UserConstructionScript`)